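; Minimap icon actor for a Palworld mod, drawn as a sprite with a dynamic material for texture and tint.
; Each tick it scales with the owning ModActor's scene capture ortho width and a live scale setting.
; A once-per-second check destroys it when its tracked Pal is dead, being captured or invalid, or its tracked object is picked, despawned or invalid.
; Icon textures load asynchronously from a path after lazy component setup.
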(event Custom|InitIconAsync
  (params (IconPath :type Soft%20Object%20Path%20Structure))
  (CallFunction|EnsureInitialized)
  (bind _returnvalue (Rendering|Material|GetTextureParameterValue (Variables|Default|GetDynMaterial) "Texture" :!class /Script/Engine.MaterialInstanceDynamic))
  (bind _astexture_2d (Utilities|Casting|CastToTexture2D _returnvalue))
  (CallFunction|SetIconTexture _astexture_2d)
  (bind _object (Utilities|AsyncLoadAsset (Class|KismetSystemLibrary|ToSoftObjRef(SoftObjPath) IconPath))
    (:Completed
      (if (Utilities|IsValid self)
        (bind _astexture_2d_2 (Utilities|Casting|CastToTexture2D _object))
        (CallFunction|SetIconTexture _astexture_2d_2)))))

(event EventTick
  (params (DeltaSeconds :type Float%20%28single-precision%29))
  (bind _self self)
  (bind _trackedpal (Variables|Default|GetTrackedPal))
  (bind _trackedgenericactor (Variables|Default|GetTrackedGenericActor))
  (bind _returnvalue (Class|PalCharacter|GetCharacterParameterComponent _trackedpal))
  (Utilities|FlowControl|Sequence
    (:then_0
      (bind _asmod_actor (Utilities|Casting|CastToModActor (Components|GetOwner)))
      (bind _returnvalue_2 (CallFunction|GetSettingFloat (Variables|/Game/Mods/YetAnotherMinimap/ModActor.ModActor_C|GetLiveConfig _asmod_actor) "Icon Scale" (Variables|Default|GetScaleSettingKey)))
      (Transformation|SetRelativeScale3D (Variables|Default|GetRenderComponent) (Math|Vector|MakeVector (* _returnvalue_2 (* (Math|Float|Clamp(Float) (Math|Float|Lerp (Variables|Default|GetBaseScale) (Variables|Default|GetZoomedScale) (Math|Float|NormalizetoRange (Variables|/Script/Engine.SceneCaptureComponent2D|GetOrthoWidth (Variables|/Game/Mods/YetAnotherMinimap/ModActor.ModActor_C|GetSzeneCaptureComponent _asmod_actor)) 5e+03 1.5e+05)) (Variables|Default|GetMinScale) (Variables|Default|GetMaxScale)) (Variables|Default|GetScaleMultiplier))) (* _returnvalue_2 (* (Math|Float|Clamp(Float) (Math|Float|Lerp (Variables|Default|GetBaseScale) (Variables|Default|GetZoomedScale) (Math|Float|NormalizetoRange (Variables|/Script/Engine.SceneCaptureComponent2D|GetOrthoWidth (Variables|/Game/Mods/YetAnotherMinimap/ModActor.ModActor_C|GetSzeneCaptureComponent _asmod_actor)) 5e+03 1.5e+05)) (Variables|Default|GetMinScale) (Variables|Default|GetMaxScale)) (Variables|Default|GetScaleMultiplier))) (* _returnvalue_2 (* (Math|Float|Clamp(Float) (Math|Float|Lerp (Variables|Default|GetBaseScale) (Variables|Default|GetZoomedScale) (Math|Float|NormalizetoRange (Variables|/Script/Engine.SceneCaptureComponent2D|GetOrthoWidth (Variables|/Game/Mods/YetAnotherMinimap/ModActor.ModActor_C|GetSzeneCaptureComponent _asmod_actor)) 5e+03 1.5e+05)) (Variables|Default|GetMinScale) (Variables|Default|GetMaxScale)) (Variables|Default|GetScaleMultiplier))))))
    (:then_1
      (Variables|Default|SetLivenessCheckTimer (+ DeltaSeconds (Variables|Default|GetLivenessCheckTimer)))
      (if (>= (+ DeltaSeconds (Variables|Default|GetLivenessCheckTimer)) 1.0)
        (Variables|Default|SetLivenessCheckTimer 0.0)
        (Utilities|FlowControl|Sequence
          (:then_0
            (if (Variables|Default|GetbHasTrackedPal)
              (if (Utilities|IsValid _trackedpal)
                (if (or (Class|PalCharacterParameterComponent|IsDead _returnvalue) (Class|PalCharacterParameterComponent|GetIsCapturedProcessing _returnvalue))
                  (Rendering|SetVisibility (Variables|Default|GetRenderComponent) false true)
                  (Actor|DestroyActor _self))
                (else
                  (Rendering|SetVisibility (Variables|Default|GetRenderComponent) false true)
                  (Actor|DestroyActor _self)))))
          (:then_1
            (if (Variables|Default|GetbHasTrackedGenericActor)
              (if (Utilities|IsValid _trackedgenericactor)
                (if (Variables|Default|GetbCheckPickedInClient)
                  (bind _aspal_level_object_obtainable (Utilities|Casting|CastToPalLevelObjectObtainable _trackedgenericactor))
                  (if (Variables|/Script/Pal.PalLevelObjectObtainable|GetbPickedInClient _aspal_level_object_obtainable)
                    (Rendering|SetVisibility (Variables|Default|GetRenderComponent) false true :!label _label)
                    (Actor|DestroyActor self))
                  (else
                    (bind _aspal_map_object (Utilities|Casting|CastToPalMapObject _trackedgenericactor))
                    (if (not (Utilities|Struct|BreakPalMapObjectPoolSpawnState (Variables|/Script/Pal.PalMapObject|GetPoolSpawnState _aspal_map_object)))
                      (goto _label))))
                (else
                  (Rendering|SetVisibility (Variables|Default|GetRenderComponent) false true)
                  (Actor|DestroyActor self))))))))))

(fn ConstructionScript)

(fn EnsureInitialized
  (bind _rendercomponent (Variables|Default|GetRenderComponent))
  (bind _rendercomponent_2 (Variables|Default|GetRenderComponent))
  (if (Variables|Default|GetbIsInitialized)
    (return)
    (else
      (Transformation|SetMobility _rendercomponent_2 "Movable")
      (Transformation|SetAbsolute _rendercomponent_2 false (Variables|Default|GetbLockRotationNorth) false)
      (Collision|SetCollisionEnabled (Variables|Default|GetRenderComponent) "NoCollision")
      (Transformation|SetRelativeLocation (Variables|Default|GetRenderComponent) (Math|Vector|MakeVector 0.0 0.0 (Variables|Default|GetHeightOffset)) false false)
      (Rendering|SetTranslucentSortPriority (Variables|Default|GetRenderComponent) (Variables|Default|GetSortPriority))
      (Rendering|Components|Sprite|SetSprite _rendercomponent "/Game/Mods/YetAnotherMinimap/TransparencyBg_Sprite.TransparencyBg_Sprite")
      (Transformation|SetRelativeRotation _rendercomponent "0, -90, 90" false false)
      (bind _returnvalue (Rendering|Material|CreateDynamicMaterialInstance _rendercomponent 0 (Variables|Default|GetIconMaterial) "None" :!class /Script/Engine.PrimitiveComponent))
      (bind _output_get (Variables|Default|SetDynMaterial _returnvalue))
      (Rendering|Material|SetMaterial _rendercomponent 0 _output_get)
      (Variables|Default|SetbIsInitialized true)
      (return))))

(fn SetIconTexture
  (params (IconTexture :type Texture%202D%20Object%20Reference))
  (bind _dynmaterial (Variables|Default|GetDynMaterial))
  (CallFunction|EnsureInitialized)
  (Rendering|Material|SetTextureParameterValue _dynmaterial "Texture" IconTexture)
  (Rendering|Material|SetVectorParameterValue _dynmaterial "TintColor" "(R=1.0,G=1.0,B=1.0,A=1.0)" :!class /Script/Engine.MaterialInstanceDynamic)
  (return))

(fn SetIconColor
  (params (Color :type Linear%20Color%20Structure))
  (Rendering|Material|SetVectorParameterValue (Variables|Default|GetDynMaterial) "TintColor" Color :!class /Script/Engine.MaterialInstanceDynamic))